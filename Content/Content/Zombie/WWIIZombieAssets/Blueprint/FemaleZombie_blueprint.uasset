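; Female zombie character Blueprint whose outfit and colors are configurable, applied in the construction script.
; Clothing switches on an enum to show one of two outfit skeletal meshes, hide the other, and bind it to the body mesh via master pose.
; ClothingColor then creates dynamic material instances to tint the hair and the selected outfit's color parameters.
; BeginPlay and Tick are empty.
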(event EventBeginPlay)

(event EventTick
  (params (DeltaSeconds :type Float%20%28single-precision%29)))

(fn ConstructionScript
  (CallFunction|Clothing)
  (CallFunction|ClothingColor))

(fn Clothing
  (bind _outfit1 (Variables|Default|GetOutfit1))
  (bind _outfit2 (Variables|Default|GetOutfit2))
  ;[1 1 1] Switch on Enum
  (switch Utilities|FlowControl|Switch|SwitchonFemaleClothing (Variables|Customization|GetClothing:)
    (:NewEnumerator1
      ;[1 1 1] Cutfit A
      (Rendering|SetVisibility _outfit1 true false)
      (Class|SkinnedMeshComponent|SetSkeletalMesh _outfit1 "/Game/Content/Zombie/WWIIZombieAssets/CharacterMesh/FemaleZombie/SK_FemaleZombie_Outfit1.SK_FemaleZombie_Outfit1" true)
      (Class|SkinnedMeshComponent|SetMasterPoseComponent _outfit1 (Variables|Character|GetMesh) false)
      (Rendering|SetVisibility (Variables|Default|GetOutfit2) false false))
    (:NewEnumerator2
      ;[1 1 1] Outfit B
      (Rendering|SetVisibility _outfit2 true false)
      (Class|SkinnedMeshComponent|SetSkeletalMesh _outfit2 "/Game/Content/Zombie/WWIIZombieAssets/CharacterMesh/FemaleZombie/SK_FemaleZombie_Outfit2.SK_FemaleZombie_Outfit2" true)
      (Class|SkinnedMeshComponent|SetMasterPoseComponent _outfit2 (Variables|Character|GetMesh) false)
      (Rendering|SetVisibility (Variables|Default|GetOutfit1) false false))))

(fn ClothingColor
  (bind _outfit1 (Variables|Default|GetOutfit1))
  (bind _outfit2 (Variables|Default|GetOutfit2))
  (bind _mesh (Variables|Character|GetMesh))
  (Utilities|FlowControl|Sequence
    (:then_0
      ;[1 1 1] HairColor
      (bind _returnvalue (Rendering|Material|CreateDynamicMaterialInstance _mesh 0 (Variables|Customization|GetHair_Mat) "None" :!class /Script/Engine.PrimitiveComponent))
      (bind _output_get (Variables|Customization|SetHair_MatIns _returnvalue))
      (Rendering|Material|SetMaterial _mesh 0 _output_get)
      (Rendering|Material|SetVectorParameterValue (Variables|Customization|GetHair_MatIns) "Hair" (Variables|Customization|GetHair_Color:) :!class /Script/Engine.MaterialInstanceDynamic))
    (:then_1
      ;[1 1 1] Switch Color on Outfit
      (switch Utilities|FlowControl|Switch|SwitchonFemaleClothing (Variables|Customization|GetClothing:)
        (:NewEnumerator1
          ;[1 1 1] Outfit1 Color
          (bind _returnvalue_2 (Rendering|Material|CreateDynamicMaterialInstance _outfit1 0 (Variables|Customization|GetOut1_Mat) "None" :!class /Script/Engine.PrimitiveComponent))
          (bind _output_get_2 (Variables|Customization|SetOut1_MatIns _returnvalue_2))
          (Rendering|Material|SetMaterial _outfit1 0 _output_get_2)
          (Rendering|Material|SetVectorParameterValue (Variables|Customization|GetOut1_MatIns) "Outfit_Over Color" (Variables|Customization|GetOutfit1_Top_Color:) :!class /Script/Engine.MaterialInstanceDynamic)
          (Rendering|Material|SetVectorParameterValue (Variables|Customization|GetOut1_MatIns) "Outfit_Under Color" (Variables|Customization|GetOutfit1_Under_Color:) :!class /Script/Engine.MaterialInstanceDynamic))
        (:NewEnumerator2
          ;[1 1 1] Outfit2 Color
          (bind _returnvalue_3 (Rendering|Material|CreateDynamicMaterialInstance _outfit2 0 (Variables|Customization|GetOut2_mat) "None" :!class /Script/Engine.PrimitiveComponent))
          (bind _output_get_3 (Variables|Customization|SetOut2_matIns _returnvalue_3))
          (Rendering|Material|SetMaterial _outfit2 0 _output_get_3)
          (Rendering|Material|SetVectorParameterValue (Variables|Customization|GetOut2_matIns) "Outfit Color" (Variables|Customization|GetOutfit2_color:) :!class /Script/Engine.MaterialInstanceDynamic))))))