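; Customizable male zombie Blueprint that sets up outfit and colors in its Construction Script, with no gameplay logic.
; Clothing switches on an enum to show and assign vest, trench coat or combined skeletal meshes, slaved to the body via master pose.
; Color creates dynamic material instances to tint hair, pants, shoes and the selected outfit.
; The combined case leaves single-garment visibility untouched, and the single cases never hide the combined mesh.
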(event EventBeginPlay)

(event EventTick
  (params (DeltaSeconds :type Float%20%28single-precision%29)))

(fn ConstructionScript
  (CallFunction|Clothing)
  (CallFunction|Color))

(fn Clothing
  (bind _both_tri_ (Variables|Default|GetBoth%28tri%29))
  (bind _vest (Variables|Default|GetVest))
  (bind _trench_coat (Variables|Default|GetTrench_Coat))
  ;[1 1 1] Switch on Enum
  (switch Utilities|FlowControl|Switch|SwitchonMaleClothing (Variables|Customization|GetClothing:)
    (:NewEnumerator1
      ;[1 1 1] Vest
      (Rendering|SetVisibility _vest true false)
      (Class|SkinnedMeshComponent|SetSkeletalMesh _vest "/Game/Content/Zombie/WWIIZombieAssets/CharacterMesh/MaleZombie/SK_MaleZombie_Vest.SK_MaleZombie_Vest" true)
      (Class|SkinnedMeshComponent|SetMasterPoseComponent _vest (Variables|Character|GetMesh) false)
      (Rendering|SetVisibility (Variables|Default|GetTrench_Coat) false false))
    (:NewEnumerator2
      ;[1 1 1] Coat
      (Rendering|SetVisibility _trench_coat true false)
      (Class|SkinnedMeshComponent|SetSkeletalMesh _trench_coat "/Game/Content/Zombie/WWIIZombieAssets/CharacterMesh/MaleZombie/SK_MaleZombie_TrenchCoat.SK_MaleZombie_TrenchCoat" true)
      (Class|SkinnedMeshComponent|SetMasterPoseComponent _trench_coat (Variables|Character|GetMesh) false)
      (Rendering|SetVisibility (Variables|Default|GetVest) false false))
    (:NewEnumerator3
      ;[1 1 1] Coat&Vest
      (Rendering|SetVisibility _both_tri_ true false)
      (Class|SkinnedMeshComponent|SetSkeletalMesh _both_tri_ "/Game/Content/Zombie/WWIIZombieAssets/CharacterMesh/MaleZombie/SK_MaleZombie_Tri.SK_MaleZombie_Tri" true)
      (Class|SkinnedMeshComponent|SetMasterPoseComponent _both_tri_ (Variables|Character|GetMesh) false))))

(fn Color
  (bind _vest (Variables|Default|GetVest))
  (bind _trench_coat (Variables|Default|GetTrench_Coat))
  (bind _mesh (Variables|Character|GetMesh))
  (bind _both_tri_ (Variables|Default|GetBoth%28tri%29))
  (bind _both_tri__2 (Variables|Default|GetBoth%28tri%29))
  (bind _mesh_2 (Variables|Character|GetMesh))
  (Utilities|FlowControl|Sequence
    (:then_0
      ;[1 1 1] Hair Color
      (bind _returnvalue (Rendering|Material|CreateDynamicMaterialInstance _mesh_2 0 (Variables|Customization|GetHair_Mat) "None" :!class /Script/Engine.PrimitiveComponent))
      (bind _output_get (Variables|Customization|SetHair_MatIns _returnvalue))
      (Rendering|Material|SetMaterial _mesh_2 0 _output_get)
      (Rendering|Material|SetVectorParameterValue (Variables|Customization|GetHair_MatIns) "Hair" (Variables|Customization|GetHair_Color:) :!class /Script/Engine.MaterialInstanceDynamic)
      ;[1 1 1] Bottom
      (bind _returnvalue_2 (Rendering|Material|CreateDynamicMaterialInstance _mesh 1 (Variables|Customization|GetBottom_Mat) "None" :!class /Script/Engine.PrimitiveComponent))
      (bind _output_get_2 (Variables|Customization|SetBottom_MatIns _returnvalue_2))
      (Rendering|Material|SetMaterial _mesh 1 _output_get_2)
      (Rendering|Material|SetVectorParameterValue (Variables|Customization|GetBottom_MatIns) "Pants" (Variables|Customization|GetBotom_Color:) :!class /Script/Engine.MaterialInstanceDynamic)
      (Rendering|Material|SetVectorParameterValue (Variables|Customization|GetBottom_MatIns) "Shoes" (Variables|Customization|GetShoes_Color:) :!class /Script/Engine.MaterialInstanceDynamic))
    (:then_1
      ;[1 1 1] Switch Color On outfit
      (switch Utilities|FlowControl|Switch|SwitchonMaleClothing (Variables|Customization|GetClothing:)
        (:NewEnumerator1
          ;[1 1 1] Vest Color
          (bind _returnvalue_3 (Rendering|Material|CreateDynamicMaterialInstance _vest 0 (Variables|Customization|GetVest_Mat) "None" :!class /Script/Engine.PrimitiveComponent))
          (bind _output_get_3 (Variables|Customization|SetVest_MatIns _returnvalue_3))
          (Rendering|Material|SetMaterial _vest 0 _output_get_3)
          (Rendering|Material|SetVectorParameterValue (Variables|Customization|GetVest_MatIns) "Vest" (Variables|Customization|GetVest_Color:) :!class /Script/Engine.MaterialInstanceDynamic))
        (:NewEnumerator2
          ;[1 1 1] Coat Color
          (bind _returnvalue_4 (Rendering|Material|CreateDynamicMaterialInstance _trench_coat 0 (Variables|Customization|GetCoat_Mat) "None" :!class /Script/Engine.PrimitiveComponent))
          (bind _output_get_4 (Variables|Customization|SetCoat_MatIns _returnvalue_4))
          (Rendering|Material|SetMaterial _trench_coat 0 _output_get_4)
          (Rendering|Material|SetVectorParameterValue (Variables|Customization|GetCoat_MatIns) "Coat_Color" (Variables|Customization|GetCoat_Color) :!class /Script/Engine.MaterialInstanceDynamic))
        (:NewEnumerator3
          ;[1 1 1] (Both)Vest Color
          (bind _returnvalue_5 (Rendering|Material|CreateDynamicMaterialInstance _both_tri_ 0 (Variables|Customization|GetVest_Mat) "None" :!class /Script/Engine.PrimitiveComponent))
          (bind _output_get_5 (Variables|Customization|SetVest_MatIns _returnvalue_5))
          (Rendering|Material|SetMaterial _both_tri_ 0 _output_get_5)
          (Rendering|Material|SetVectorParameterValue (Variables|Customization|GetVest_MatIns) "Vest" (Variables|Customization|GetVest_Color:) :!class /Script/Engine.MaterialInstanceDynamic)
          ;[1 1 1] (Both)Coat Color
          (bind _returnvalue_6 (Rendering|Material|CreateDynamicMaterialInstance _both_tri__2 1 (Variables|Customization|GetCoat_Mat) "None" :!class /Script/Engine.PrimitiveComponent))
          (bind _output_get_6 (Variables|Customization|SetCoat_MatIns _returnvalue_6))
          (Rendering|Material|SetMaterial _both_tri__2 1 _output_get_6)
          (Rendering|Material|SetVectorParameterValue (Variables|Customization|GetCoat_MatIns) "Coat_Color" (Variables|Customization|GetCoat_Color) :!class /Script/Engine.MaterialInstanceDynamic))))))